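; BP_Item is a physics-simulated world item whose mesh is set from ItemModelToPlace at construction, with a trigger that tracks overlap.
; PickUp shrinks the mesh on a timeline, with a DoOnce on its update playing a sound and destroying the actor after a short delay.
; Drop scales the mesh back up with its own sound.
; PrimaryAction, PrimaryUse and OldPickUp are empty stubs, and older attach, detach and impulse logic is left disconnected.
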(event `self.ReceiveBeginPlay`
  (`PrimitiveComponent.SetSimulatePhysics` (`self.ItemModel`) true))

(event `self.ReceiveTick`
  (params (DeltaSeconds :type "Float (single-precision)"))
  ;[1 1 1] Old Code
)

(event `OldPickUp`
  (params (Parent :type "SceneComponent Object Reference"))
  ;[1 1 1] Old Code
)

(event `PrimaryAction`
  (params (`Held Down` :type Boolean :default true))
  ;[1 1 1] Old Code
)

(event `PrimaryUse`
  (params (HeldDown :type Boolean :default true))
  ;[1 1 1] Old Code
)

(event `/Game/Items/BPI_Items.PickUp`
  ;[1 1 1] Old Code
  (`KismetSystemLibrary.PrintString` "ItemPicked")
  (bind (_direction _shrinktimeline) (`Timeline|Shrink`)
    (:`Update`
      (`SceneComponent.SetWorldScale3D` (`self.ItemModel`) (`KismetMathLibrary.Conv_DoubleToVector` (`KismetMathLibrary.Lerp` 1.0 0.0 _shrinktimeline)))
      (`/Engine/EditorBlueprintResources/StandardMacros.DoOnce` false
        (:`Completed`
          (`GameplayStatics.PlaySound2D` "/Engine/VREditor/Sounds/UI/Object_PickUp.Object_PickUp" 1.0 1.0 0.0 null null)
          (`KismetSystemLibrary.Delay` 0.1)
          (`self.K2_DestroyActor`))))))

(event `/Game/Items/BPI_Items.Drop`
  ;[1 1 1] Old Code
  (`KismetSystemLibrary.PrintString` "ItemDropped")
  (bind (_direction _shrinktimeline) (`Timeline|Timeline`)
    (:`Update`
      (`SceneComponent.SetWorldScale3D` (`self.ItemModel`) (`KismetMathLibrary.Conv_DoubleToVector` (`KismetMathLibrary.Lerp` 0.0 1.0 _shrinktimeline)))
      (`/Engine/EditorBlueprintResources/StandardMacros.DoOnce` false
        (:`Completed`
          (`GameplayStatics.PlaySound2D` "/Engine/VREditor/Sounds/UI/Drop_Item_From_ContentBrowser.Drop_Item_From_ContentBrowser" 1.0 1.0 0.0 null null)
          (`KismetSystemLibrary.Delay` 0.1))))))

(event `self.Trigger.OnComponentBeginOverlap`
  (params (OverlappedComponent :type "PrimitiveComponent Object Reference") (OtherActor :type "Actor Object Reference") (OtherComp :type "PrimitiveComponent Object Reference") (OtherBodyIndex :type Integer) (bFromSweep :type Boolean) (SweepResult :type "HitResult Structure (by ref)"))
  ;[1 1 1] Old Code
  (set `self.ItemOverlap` true))

(event `self.Trigger.OnComponentEndOverlap`
  (params (OverlappedComponent :type "PrimitiveComponent Object Reference") (OtherActor :type "Actor Object Reference") (OtherComp :type "PrimitiveComponent Object Reference") (OtherBodyIndex :type Integer))
  ;[1 1 1] Old Code
  (set `self.ItemOverlap` false))

(fn `UserConstructionScript`
  (`StaticMeshComponent.SetStaticMesh` (`self.ItemModel`) (`self.ItemModelToPlace`)))