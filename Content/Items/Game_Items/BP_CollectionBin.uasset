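; BP_CollectionBin is a collection bin that counts BP_Item actors placed in it and bursts into flame.
; On each CountingTrigger overlap, it loops over BP_Item actors overlapping the triggering component, setting and printing Counter.
; A count of one or more prints a success message and, after a delay, calls Incinerate, which only spawns a large fire emitter.
; A WB_Objective widget appears only if a looped item casts to BP_ThirdPersonCharacter.
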(event `self.CountingTrigger.OnComponentBeginOverlap`
  (params (OverlappedComponent :type "PrimitiveComponent Object Reference") (OtherActor :type "Actor Object Reference") (OtherComp :type "PrimitiveComponent Object Reference") (OtherBodyIndex :type Integer) (bFromSweep :type Boolean) (SweepResult :type "HitResult Structure (by ref)"))
  ;[1 1 1] CollectionBinCounter
  (for (_array_element _array_index) (`PrimitiveComponent.GetOverlappingActors` OverlappedComponent "/Game/Items/BP_Item.BP_Item_C")
    (`|ExecutionSequence`
      (:`then_0`
        (bind _output_get (set `self.Counter` (+ _array_index 1)))
        (`KismetSystemLibrary.PrintString` (`KismetStringLibrary.Conv_IntToString` _output_get))
        (if (>= _output_get 1)
          (`|ExecutionSequence`
            (:`then_0`
              (`KismetSystemLibrary.PrintString` "You did it!"))
            (:`then_1`
              (`KismetSystemLibrary.Delay` 2.0)
              (`self.Incinerate`)))))
      (:`then_1`
        (cast `/Game/ThirdPerson/Blueprints/BP_ThirdPersonCharacter` _array_element)
        (set `self.Counter` _output_get)
        (bind _returnvalue (`|CreateWidget` "/Game/Items/WB_Objective.WB_Objective_C"))
        (`UserWidget.AddToViewport` _returnvalue 0)))))

(event `Incinerate`
  ;[1 1 1] CollectionBinEmitter
  (`GameplayStatics.SpawnEmitterAtLocation` "/Game/PolygonAdventure/Particles/FX_Fire.FX_Fire" (`self.K2_GetActorLocation` (`ActorComponent.GetOwner` (`self.StaticMesh`))) (struct) (30.0 30.0 30.0)))

(fn `UserConstructionScript`)