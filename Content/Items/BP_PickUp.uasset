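; Pickup item actor that shrinks, plays a pickup sound and destroys itself when its PickUp event is called.
; The Shrink timeline scales the root toward zero, and a DoOnce on its first update plays the sound, then destroys the actor after a short delay, independent of timeline completion.
; The construction script applies the ItemModelToPlace mesh to ItemModel, so one Blueprint can show different items.
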(event `/Game/Items/BPI_Items.PickUp`
  (`KismetSystemLibrary.PrintString` "ItemPicked")
  (bind (_direction _shrinktimeline) (`Timeline|Shrink`)
    (:`Update`
      (`SceneComponent.SetWorldScale3D` (`self.DefaultSceneRoot`) (`KismetMathLibrary.Conv_DoubleToVector` (`KismetMathLibrary.Lerp` 1.0 0.0 _shrinktimeline)))
      (`/Engine/EditorBlueprintResources/StandardMacros.DoOnce` false
        (:`Completed`
          (`GameplayStatics.PlaySound2D` "/Engine/VREditor/Sounds/UI/Object_PickUp.Object_PickUp" 1.0 1.0 0.0 null null)
          (`KismetSystemLibrary.Delay` 0.1)
          (`self.K2_DestroyActor`))))))

(fn `UserConstructionScript`
  (`StaticMeshComponent.SetStaticMesh` (`self.ItemModel`) (`self.ItemModelToPlace`)))