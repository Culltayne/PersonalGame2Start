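; BP_Enemy is an enemy Blueprint with draft logic for losing health and dying, none of which is connected.
; Its BeginPlay and TakeDamage events are empty, so the taunt message and damage chain never run.
; The unwired damage chain subtracts from Health, prints the result, and uses CheckIfAlive to destroy the actor once health is no longer above zero.
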(event `self.ReceiveBeginPlay`)

(event `TakeDamage`
  (params (by :type "Float (double-precision)" :default 0.2)))

(fn `CheckIfAlive`
  (params (Health :type "Float (double-precision)"))
  (returns (IsAlive :type Boolean))
  (return (> Health 0.0)))

(fn `UserConstructionScript`)